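; Base character Blueprint that supplies aim offset updates and weapon animation settings on top of its parent class.
; Each tick on authority, it interpolates the aim offset toward the control-minus-actor rotation delta, clamps yaw and pitch, and passes them to ServerUpdateAimOffset.
; An initializer stores weapon animation type, right-hand weapon position and reload montage options, exposed through simple getters.
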(event `self.ReceiveBeginPlay`
  ;[1 1 1] EVENT BEGIN PLAY
  (`parent.ReceiveBeginPlay`))

(event `self.ReceiveTick`
  (params (DeltaSeconds :type "Float (single-precision)"))
  ;[1 1 1] EVENT TICK
  (bind _output_get (set `self.Basic Base Delta Second Time` DeltaSeconds))
  (`parent.ReceiveTick` _output_get)
  (`/Engine/EditorBlueprintResources/ActorMacros.Switch Has Authority`
    (:`Authority`
      (`self.UpdateAimOffSet`))))

(event `UpdateAimOffSet`
  (bind (_aimyaw _aimpitch) (`self.GetAimOffSetValues`))
  ;[1 1 1] EVENT TICK
  (`self.ServerUpdateAimOffset` (`KismetMathLibrary.FClamp` (.yaw (`KismetMathLibrary.RInterpTo` (`KismetMathLibrary.MakeRotator` 0.0 _aimpitch _aimyaw) (`KismetMathLibrary.NormalizedDeltaRotator` (`self.GetControlRotation`) (`self.K2_GetActorRotation`)) (`self.Basic Base Delta Second Time`) 25.0)) -90.0 90.0) (`KismetMathLibrary.FClamp` (.pitch (`KismetMathLibrary.RInterpTo` (`KismetMathLibrary.MakeRotator` 0.0 _aimpitch _aimyaw) (`KismetMathLibrary.NormalizedDeltaRotator` (`self.GetControlRotation`) (`self.K2_GetActorRotation`)) (`self.Basic Base Delta Second Time`) 25.0)) -75.0 75.0)))

(fn `Get New Reload Animation Montage`
  (returns (`New Reload Animation Montage` :type "AnimMontage Object Reference"))
  (return (`self.New Reload Animation Montage`)))

(fn `Get Use Default Reload Animation`
  (returns (`Use Default Reload Animation? ` :type Boolean))
  (return (`self.Use Default Reload Animation? `)))

(fn `Get Weapon Animation Type`
  (returns (WeaponAnimationType :type "/Game/TPSFPS/Blueprints/BASIC_BaseCharacter/Data/ENUM_BASIC_WeaponAnimType Enum"))
  (return (`self.Weapon Animation Type`)))

(fn `Get Weapon Position In Right Hand`
  (returns (`3RDPP Weapon Position in Right Hand` :type "Vector Structure"))
  (return (`self.Weapon Position In Right Hand`)))

(fn `Initialize Basic Base Properties`
  (params (`Weapon Animation Type` :type "/Game/TPSFPS/Blueprints/BASIC_BaseCharacter/Data/ENUM_BASIC_WeaponAnimType Enum" :default "NewEnumerator0") (`Weapon Position In Right Hand` :type "Vector Structure") (`Use Default Reload Animation? ` :type Boolean) (`New Reload Animation Montage` :type "AnimMontage Object Reference"))
  (set `self.Weapon Animation Type` `Weapon Animation Type`)
  (set `self.Weapon Position In Right Hand` `Weapon Position In Right Hand`)
  (set `self.Use Default Reload Animation? ` `Use Default Reload Animation? `)
  (set `self.New Reload Animation Montage` `New Reload Animation Montage`))

(fn `UserConstructionScript`
  (`parent.UserConstructionScript`))