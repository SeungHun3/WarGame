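; AI controller for BP_Enemy that runs BT_Enemy and supplies its blackboard.
; On begin play it copies the pawn's two patrol point locations and crouch flag into blackboard keys.
; Perception updates store a sensed player character in Player_ActorKey and clear it when sensing fails, while forgotten targets only print a debug message.
; ChangeAttack exposes a setter for the CanAttack key.
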(event `self.AIPerception.OnTargetPerceptionUpdated`
  (params (Actor :type "Actor Object Reference") (Stimulus :type "AIStimulus Structure"))
  (bind _asbp_basic_tpsfpscharacter (cast `/Game/TPSFPS/Blueprints/BASIC_TPSFPSCharacter/BP_BASIC_TPSFPSCharacter` Actor))
  (if Stimulus_bSuccessfullySensed
    (`self.Check Player` _asbp_basic_tpsfpscharacter)
    (else
      (`self.Check Player` null))))

(event `self.AIPerception.OnTargetPerceptionForgotten`
  (params (Actor :type "Actor Object Reference"))
  (`KismetSystemLibrary.PrintString` "타겟 놓침"))

(event `self.ReceiveBeginPlay`
  (`KismetSystemLibrary.PrintString` "//Enemy Controller Begin")
  (`self.RunBehaviorTree` "/Game/TPSFPS/Blueprints/AI_Folder/BT_Enemy.BT_Enemy")
  (`self.Init_PatrolPoint`))

(event `self.AIPerception.OnPerceptionUpdated`
  (params (UpdatedActors :type "Array of Actor Object Reference (by ref)")))

(fn `ChangeAttack`
  (params (CanAttack :type Boolean))
  (`BlackboardComponent.SetValueAsBool` (`AIBlueprintHelperLibrary.GetBlackboard` null) "CanAttack" CanAttack))

(fn `Check Player`
  (params (SensedActor :type "Actor Object Reference"))
  (`BlackboardComponent.SetValueAsObject` (`AIBlueprintHelperLibrary.GetBlackboard` null) "Player_ActorKey" SensedActor))

(fn `Init_PatrolPoint`
  (bind _returnvalue (`AIBlueprintHelperLibrary.GetBlackboard` null))
  (bind _asbp_enemy (cast `/Game/TPSFPS/Blueprints/AI_Folder/BP_Enemy` (`self.K2_GetPawn`)))
  (bind _output_get (set `self.EnemyPawn` _asbp_enemy))
  (bind _patrol_location (`/Game/TPSFPS/Blueprints/AI_Folder/BP_Enemy.Patrol_Location` _output_get))
  (`BlackboardComponent.SetValueAsVector` _returnvalue "Patrol_1" (`self.K2_GetActorLocation` (`|GetArrayItem` _patrol_location)))
  (`BlackboardComponent.SetValueAsVector` _returnvalue "Patrol_2" (`self.K2_GetActorLocation` (`|GetArrayItem` _patrol_location 1)))
  (`BlackboardComponent.SetValueAsBool` _returnvalue "IsCrouch" (`/Game/TPSFPS/Blueprints/AI_Folder/BP_Enemy.IsCrouch` _output_get)))

(fn `UserConstructionScript`)