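; BP_Enemy is an AI-controlled gun enemy that fires bursts at a given player and, when health runs out, is unpossessed and flagged dead.
; The construction script reads its child-actor weapon to place the muzzle effect and derive slowed fire and burst timings.
; Attack uses those timings to gate hitscan shots with random spread, spawning surface-matched effects and decals and calling ApplyDamage on player-character hits.
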(event `self.ReceiveBeginPlay`
  (set `self.CurrentHealth` 100.0))

(event `self.ReceiveAnyDamage`
  (params (Damage :type "Float (single-precision)") (DamageType :type "DamageType Object Reference") (InstigatedBy :type "Controller Object Reference") (DamageCauser :type "Actor Object Reference"))
  (bind _returnvalue (`AIBlueprintHelperLibrary.GetAIController` self))
  (bind _output_get (set `self.CurrentHealth` (- (`self.CurrentHealth`) Damage)))
  (if (<= _output_get 0.0)
    (`/Engine/EditorBlueprintResources/StandardMacros.DoOnce` false
      (:`Completed`
        (`/Engine/EditorBlueprintResources/StandardMacros.IsValid` _returnvalue
          (:`Is Valid`
            (`Controller.UnPossess` _returnvalue)
            (set `self.bCanBeDamaged` false)
            (set `self.IsDead` true)))))))

(event `self.ReceiveTick`
  (params (DeltaSeconds :type "Float (single-precision)")))

(event `Reset_Burst`
  (`KismetSystemLibrary.Delay` (`self.Burst_Delay`))
  (set `self.Burst_Count` 0))

(event `StartMuzzle`
  (bind _ps_defaultmuzzle (`self.PS_DefaultMuzzle`))
  (`ActorComponent.SetActive` _ps_defaultmuzzle true false)
  (`KismetSystemLibrary.Delay` 0.2)
  (`ActorComponent.SetActive` _ps_defaultmuzzle false false))

(fn `Attack`
  (params (Player :type "Actor Object Reference"))
  (bind _currentweapon (`self.CurrentWeapon`))
  (bind ((`MuzzleSFXSocket_213_7055603F460EF14A93623396B0E92A38` _muzzlesfxsocket) (`TrailSFX_144_6C7956D143EE9DF3DD179A919EF7EAF1` _trailsfx) (`TrailSpeed_153_08F00C6F4C92B70D74D5EAB3F8A2CD28` _trailspeed) (`TrailScale_158_3F8331E1498D8B2E2DBA9C9E99E91F6F` _trailscale) (`SurfaceHitSFXArray_227_2896D8DF4D7F81D292868AA0BA1939F3` _surfacehitsfxarray) (`SurfaceHitDecalArray_235_EB09D24343C93538339F17B4F28E817A` _surfacehitdecalarray)) (break `/Game/TPSFPS/Blueprints/COMMON_WeaponSystem/Data/STR_SFXWeaponProperties` (`/Game/TPSFPS/Blueprints/COMMON_WeaponSystem/BP_BaseWeapon.SFX Weapon Properties` _currentweapon)))
  (bind _returnvalue (`SceneComponent.GetSocketLocation` (`/Game/TPSFPS/Blueprints/COMMON_WeaponSystem/BP_BaseWeapon.WeaponSkeletalMesh` _currentweapon) _muzzlesfxsocket))
  (`self.Attack_Delay`
    (:`Shoot`
      (`|ExecutionSequence`
        (:`then_0`
          (`self.StartMuzzle`))
        (:`then_1`)
        (:`then_2`
          (bind _outhit (`KismetSystemLibrary.LineTraceSingleForObjects` _returnvalue (`KismetMathLibrary.MakeVector` (+ (.x (+ _returnvalue (* (`KismetMathLibrary.GetForwardVector` (`KismetMathLibrary.FindLookAtRotation` _returnvalue (`self.K2_GetActorLocation` Player))) (`/Game/TPSFPS/Blueprints/COMMON_WeaponSystem/BP_BaseWeapon.ShootingMaxDistance` (`self.CurrentWeapon`))))) (`KismetMathLibrary.RandomFloatInRange` -5000.0 5000.0)) (+ (.y (+ _returnvalue (* (`KismetMathLibrary.GetForwardVector` (`KismetMathLibrary.FindLookAtRotation` _returnvalue (`self.K2_GetActorLocation` Player))) (`/Game/TPSFPS/Blueprints/COMMON_WeaponSystem/BP_BaseWeapon.ShootingMaxDistance` (`self.CurrentWeapon`))))) (`KismetMathLibrary.RandomFloatInRange` -5000.0 5000.0)) (+ (.z (+ _returnvalue (* (`KismetMathLibrary.GetForwardVector` (`KismetMathLibrary.FindLookAtRotation` _returnvalue (`self.K2_GetActorLocation` Player))) (`/Game/TPSFPS/Blueprints/COMMON_WeaponSystem/BP_BaseWeapon.ShootingMaxDistance` (`self.CurrentWeapon`))))) (`KismetMathLibrary.RandomFloatInRange` -50.0 50.0))) (`self.Object Types`)))
          (bind (_bblockinghit _binitialoverlap _time _distance _location _impactpoint _normal _impactnormal _physmat _hitactor _hitcomponent _hitbonename) (`GameplayStatics.BreakHitResult` _outhit))
          (`/Engine/EditorBlueprintResources/StandardMacros.IsValid` _hitactor
            (:`Is Valid`
              (for _array_element _surfacehitsfxarray
                (bind (_surfacephystype _sfx) (break `/Game/TPSFPS/Blueprints/COMMON_WeaponSystem/Data/STR_SFXBasedonSurfaceDesc` _array_element))
                (bind _returnvalue_2 (`GameplayStatics.GetSurfaceType` _outhit))
                (if (`|EnumEquality` _surfacephystype _returnvalue_2)
                  (if (`|EnumEquality` _returnvalue_2 "SurfaceType4")
                    (bind _asbp_basic_tpsfpscharacter (cast `/Game/TPSFPS/Blueprints/BASIC_TPSFPSCharacter/BP_BASIC_TPSFPSCharacter` _hitactor))
                    (`GameplayStatics.SpawnEmitterAttached` _sfx (`/Game/TPSFPS/Blueprints/BASIC_FPSCharacter/BP_BASIC_FPSCharacter.FPSCamera` _asbp_basic_tpsfpscharacter) "None" (0.0 0.0 0.0) (struct) (1.0 1.0 1.0) "SnapToTarget")
                    (else
                      (`GameplayStatics.SpawnEmitterAtLocation` _sfx _location (`KismetMathLibrary.MakeRotFromX` _normal))))))
              (for _array_element_2 _surfacehitdecalarray
                (bind (_surfacetype _decal) (break `/Game/TPSFPS/Blueprints/COMMON_WeaponSystem/Data/STR_DecalBaseonSurfaceDesc` _array_element_2))
                (if (`|EnumEquality` _surfacetype (`GameplayStatics.GetSurfaceType` _outhit))
                  (bind (_returnvalue_roll _returnvalue_pitch _returnvalue_yaw) (`KismetMathLibrary.BreakRotator` (`KismetMathLibrary.MakeRotFromX` _normal)))
                  (`GameplayStatics.SpawnDecalAtLocation` _decal (6.0 6.0 6.0) _location (`KismetMathLibrary.MakeRotator` (+ _returnvalue_roll 180.0) (+ _returnvalue_pitch 180.0) _returnvalue_yaw) 10.0)))
              (bind _asbp_basic_tpsfpscharacter_2 (cast `/Game/TPSFPS/Blueprints/BASIC_TPSFPSCharacter/BP_BASIC_TPSFPSCharacter` _hitactor))
              (`GameplayStatics.ApplyDamage` _asbp_basic_tpsfpscharacter_2))))))))

(fn `UserConstructionScript`
  (bind _currentweapon (`self.CurrentWeapon`))
  (bind _weaponskeletalmesh (`/Game/TPSFPS/Blueprints/COMMON_WeaponSystem/BP_BaseWeapon.WeaponSkeletalMesh` _currentweapon))
  (bind ((`MuzzleSFX_115_95BEBCD249DB759201852D9FEB56DA7C` _muzzlesfx) (`MuzzleSFXSocket_213_7055603F460EF14A93623396B0E92A38` _muzzlesfxsocket)) (break `/Game/TPSFPS/Blueprints/COMMON_WeaponSystem/Data/STR_SFXWeaponProperties` (`/Game/TPSFPS/Blueprints/COMMON_WeaponSystem/BP_BaseWeapon.SFX Weapon Properties` _currentweapon)))
  (bind ((`FireRate_200_51E05BA54DB5D1B7752FB29E5808E3F4` _firerate) (`BurstFireShotsBeforePause_205_BE0BB99B4BE3FF89BEB1F7A80BFDC8C3` _burstfireshotsbeforepause) (`BurstFirePause_206_5588FDE043A4E22E8AC096A9807D0C05` _burstfirepause)) (break `/Game/TPSFPS/Blueprints/COMMON_WeaponSystem/Data/STR_BasicWeaponProperties` (`/Game/TPSFPS/Blueprints/COMMON_WeaponSystem/BP_BaseWeapon.Basic Weapon Properties` (`self.CurrentWeapon`))))
  (bind _asbp_base_weapon (cast `/Game/TPSFPS/Blueprints/COMMON_WeaponSystem/BP_BaseWeapon` (`ChildActorComponent.ChildActor` (`self.BP_BASIC_WPN_FPS_AssaultRifleBurst`))))
  (set `self.CurrentWeapon` _asbp_base_weapon)
  (`SceneComponent.K2_SetWorldLocationAndRotation` (`self.PS_DefaultMuzzle`) (`SceneComponent.GetSocketLocation` _weaponskeletalmesh _muzzlesfxsocket) (`SceneComponent.GetSocketRotation` _weaponskeletalmesh _muzzlesfxsocket) false false)
  (set `self.Fire_Delay` (* 1.5 (/ 1.0 (/ (`KismetMathLibrary.Conv_IntToDouble` _firerate) 60.0))))
  (set `self.FireBurst` _burstfireshotsbeforepause)
  (set `self.Burst_Delay` (* _burstfirepause 2.0)))