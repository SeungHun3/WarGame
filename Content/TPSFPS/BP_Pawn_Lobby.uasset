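; BP_Pawn_Lobby is a lobby pawn, apparently for VR, that mainly drives a test HUD.
; BeginPlay adds WBP_CommonMainHUD to the viewport and prints the platform name.
; The Shot input swaps visibility between the HUD's HMD test and boundary panels, while two pad inputs only print debug text.
; Disconnected leftover logic would poll for HMD position, save it to the game instance and open Main_Level.
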(event `self.ReceiveBeginPlay`
  (bind _returnvalue (`|CreateWidget` "/Game/TPSFPS/Blueprints/COMMON_HUD/WBP_CommonMainHUD.WBP_CommonMainHUD_C"))
  (bind _output_get (set `self.MainHud` _returnvalue))
  (`UserWidget.AddToViewport` _output_get 0)
  (`KismetSystemLibrary.PrintString` (`GameplayStatics.GetPlatformName`)))

(event `InputAction|pad1`
  (params (Key :type "Key Structure"))
  (:`Pressed`
    (`KismetSystemLibrary.PrintString` "// 1번")))

(event `InputAction|Shot`
  (params (Key :type "Key Structure"))
  (bind _mainhud (`self.MainHud`))
  (bind _wb_hmd_test (`/Game/TPSFPS/Blueprints/COMMON_HUD/WBP_CommonMainHUD.WB_HMD_Test` _mainhud))
  (bind _wb_bound (`/Game/TPSFPS/Blueprints/COMMON_HUD/WBP_CommonMainHUD.WB_Bound` _mainhud))
  (:`Pressed`
    (`/Engine/EditorBlueprintResources/StandardMacros.IsValid` _mainhud
      (:`Is Valid`
        (if (`Widget.IsVisible` _wb_hmd_test)
          (`Widget.SetVisibility` _wb_hmd_test "Collapsed")
          (`Widget.SetVisibility` _wb_bound "Visible")
          (else
            (`Widget.SetVisibility` _wb_bound "Collapsed")
            (`Widget.SetVisibility` _wb_hmd_test "Visible")))))))

(event `InputAction|pad2`
  (params (Key :type "Key Structure"))
  (:`Pressed`
    (`KismetSystemLibrary.PrintString` "// 2번")))

(fn `UserConstructionScript`)